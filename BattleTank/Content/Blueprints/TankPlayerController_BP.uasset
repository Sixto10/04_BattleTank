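; Player controller for the tank pawn that feeds it an aim point from a fixed on-screen spot.
; Every tick it deprojects a point at horizontal screen center and a fixed pixel height, then runs a long visibility trace from the tank camera along that direction.
; The trace's hit location goes to the tank's AimAtPoint without a hit check, and the trace is debug-drawn each frame.
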(event EventTick
  (params (DeltaSeconds :type Float%20%28single-precision%29))
  (bind _astank_bp (Utilities|Casting|CastToTank_BP (Pawn|GetControlledPawn)))
  (bind _outhit (Collision|LineTraceByChannel (Transformation|GetWorldLocation (Variables|/Game/Tank/Tank_BP.Tank_BP_C|GetCamera _astank_bp)) (+ (Transformation|GetWorldLocation (Variables|/Game/Tank/Tank_BP.Tank_BP_C|GetCamera _astank_bp)) (* (.WorldDirection (Class|GameplayStatics|DeprojectScreentoWorld self (Math|Vector2D|MakeVector2D (.X (Math|Vector2D|BreakVector2D (/ (Viewport|GetViewportSize) 2.0))) 1.5e+02))) 1e+06)) "TraceTypeQuery1" true 0 "ForOneFrame" false))
  (Default|AimatPoint _astank_bp (.location _outhit)))

(event EventBeginPlay)

(fn ConstructionScript)