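; Player-drivable tank pawn Blueprint that aims, fires and drives on two tracks.
; Input feeds the movement component through either fly-by-wire intents or manual per-track throttles, while aim axes rotate the camera spring arm container.
; Movement and aiming components raise request events that the Blueprint forwards to the tracks, turret and barrel.
; BeginPlay sets low-friction tracks, the barrel reference and starting ammo; Tick pushes health into a widget bar.
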(event EventBeginPlay
  ;[1 1 1] Setup here as construction may be too early
  (Utilities|FlowControl|Sequence
    (:then_0
      (Class|PrimitiveComponent|SetPhysMaterialOverride (Variables|Default|GetLeft%20Track) "/Game/Tank/LowFriction.LowFriction"))
    (:then_1
      (Class|PrimitiveComponent|SetPhysMaterialOverride (Variables|Default|GetRight%20Track) "/Game/Tank/LowFriction.LowFriction"))
    (:then_2
      (Class|TankAimingComponent|SetBarrelReference (Variables|Default|GetTankAimingComponent) (Variables|Default|GetBarrel)))
    (:then_3
      (Class|Tank|AddAmmo 10))))

(event EventTick
  (params (DeltaSeconds :type Float%20%28single-precision%29))
  ;[1 1 1] Bind Tank Health to Widget TODO Review
  (bind _ashealth_bar (Utilities|Casting|CastToHealthBar (UserInterface|GetUserWidgetObject (Variables|Default|GetHealth%20Bar))))
  (Variables|/Game/Tank/HealthBar.HealthBar_C|SetProgress _ashealth_bar (Class|Tank|GetHealthPercent)))

(event OnLeftThrottleRequest(TankMovementComponent)
  (params (Throttle :type Float%20%28single-precision%29))
  ;[1 1 1] Tank Track Bindings
  (Class|TankTrack|SetThrottle (Variables|Default|GetLeft%20Track) Throttle))

(event OnRightThrottleRequest(TankMovementComponent)
  (params (Throttle :type Float%20%28single-precision%29))
  ;[1 1 1] Tank Track Bindings
  (Class|TankTrack|SetThrottle (Variables|Default|GetRight%20Track) Throttle))

(event OnTurretRotateRequest(TankAimingComponent)
  (params (Speed :type Float%20%28single-precision%29))
  ;[1 1 1] Aiming Motor Bindings
  (Class|TankTurret|Rotate (Variables|Default|GetTankTurret) Speed))

(event OnBarrelElevateRequest(TankAimingComponent)
  (params (Speed :type Float%20%28single-precision%29))
  ;[1 1 1] Aiming Motor Bindings
  (Class|TankBarrel|Elevate (Variables|Default|GetBarrel) Speed))

(event Input|ActionEvents|InputActionFire
  (params (Key :type Key%20Structure :default "AnyKey"))
  ;[1 1 1] FBW Aiming & Firing Input Binding
  (:Pressed
    (Class|Tank|Fire)))

(event Input|AxisEvents|InputAxisLeftTrackThrottle
  (params (AxisValue :type Float%20%28single-precision%29))
  ;[1 1 1] Manual Driving Input Binding
  (Class|TankMovementComponent|DriveLeftTrack (Variables|Default|GetTankMovementComponent) AxisValue))

(event Input|AxisEvents|InputAxisAimAzimuth
  (params (AxisValue :type Float%20%28single-precision%29))
  ;[1 1 1] FBW Aiming & Firing Input Binding
  (Transformation|AddLocalRotation (Variables|Default|GetSpringArmContainer) (Math|Rotator|MakeRotator 0.0 0.0 (* AxisValue (Utilities|Time|GetWorldDeltaSeconds) 1e+02)) false false))

(event Input|AxisEvents|InputAxisAimElevation
  (params (AxisValue :type Float%20%28single-precision%29))
  ;[1 1 1] FBW Aiming & Firing Input Binding
  (Transformation|AddLocalRotation (Variables|Default|GetSpringArmContainer) (Math|Rotator|MakeRotator 0.0 (* AxisValue (Utilities|Time|GetWorldDeltaSeconds) 1e+02) 0.0) false false))

(event Input|AxisEvents|InputAxisRightTrackThrottle
  (params (AxisValue :type Float%20%28single-precision%29))
  ;[1 1 1] Manual Driving Input Binding
  (Class|TankMovementComponent|DriveRightTrack (Variables|Default|GetTankMovementComponent) AxisValue))

(event Input|AxisEvents|InputAxisMoveForward
  (params (AxisValue :type Float%20%28single-precision%29))
  ;[1 1 1] FBW Driving Input Bindings
  (Class|TankMovementComponent|IntendMoveForward (Variables|Default|GetTankMovementComponent) AxisValue))

(event Input|AxisEvents|InputAxisTurnRight
  (params (AxisValue :type Float%20%28single-precision%29))
  ;[1 1 1] FBW Driving Input Bindings
  (Class|TankMovementComponent|IntendTurnRight (Variables|Default|GetTankMovementComponent) AxisValue))

(fn ConstructionScript)